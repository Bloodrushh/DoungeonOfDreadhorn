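; Base enemy Blueprint that handles attack playback and shows a text indicator for attack notifications.
; StartAttack plays a skeleton attack animation directly on the mesh, then calls FinishAttack after a fixed delay, a temporary stand-in for an anim notify.
; The TextRender starts hidden and is shown or hidden through ToggleAttackNotifaction.
; Death and damage hooks are stubs, with damage only switching on the attack without further action.
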(event `self.OnDiedBP`)

(event `self.ReceiveBeginPlay`
  (`SceneComponent.SetVisibility` (`self.TextRender`) false false))

(event `self.OnDamageTakenBP`
  (params (Amount :type Integer) (Attack :type "EAttack Enum" :default "Dexterous"))
  (switch `EAttack` Attack))

(event `self.StartAttack`
  ;[1 1 1] Simulate anim_notify event. TODO: Call it from animBP
  (`KismetSystemLibrary.PrintString` "BP_EnemyBase::StartAttack")
  (`SkeletalMeshComponent.PlayAnimation` (`self.Mesh`) "/Game/ModularCharacterSkeletonArcher/Animations/Skeleton_Anim_Attack01.Skeleton_Anim_Attack01" false)
  (`KismetSystemLibrary.Delay` 2.0)
  (`self.FinishAttack`))

(event `self.ToggleAttackNotifaction`
  (params (bEnable :type Boolean))
  (`SceneComponent.SetVisibility` (`self.TextRender`) bEnable false))

(fn `UserConstructionScript`)