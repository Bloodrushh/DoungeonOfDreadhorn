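; BP_EventTriggerFight_Base is a base Blueprint for fight event triggers, with hooks for enemy spawning, enemy death and event completion.
; OnEnemyDied only forwards the dead enemy to the parent implementation, while SpawnEnemies and the processed and finished events perform no actions.
; An unconnected loop would spawn BP_Enemy_01 at each spawn point, passing it the trigger and player pawn, but it never runs.
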(event `self.OnEventProcessedBP`
  (params (bResult :type Boolean) (Difference :type Integer))
  (if bResult
    _))

(event `self.OnEventFinishedBP`)

(event `self.OnEnemyDied`
  (params (Enemy :type "EnemyBase Object Reference"))
  (`parent.OnEnemyDied` Enemy))

(event `self.SpawnEnemies`)

(fn `UserConstructionScript`)