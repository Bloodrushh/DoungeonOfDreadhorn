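; Base Blueprint for trap event triggers in the dungeon, which sends the player to the table when triggered.
; OnTriggered calls the parent, prints a debug string, then after a short delay calls MovePlayerIntoTable on the DungeonManager.
; The event-processed, finish and disappear events have no effect.
; Unconnected leftover nodes cover trap event initiation, a health change, starting an enemy fight and finishing the event.
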(event `self.OnTriggered`
  (params (TriggeredActor :type "Actor Object Reference"))
  (`parent.OnTriggered` TriggeredActor)
  (`KismetSystemLibrary.PrintString` "OmTrigerred")
  (`KismetSystemLibrary.Delay` 0.2)
  (`DungeonManager.MovePlayerIntoTable` (`self.DungeonManager`)))

(event `self.OnEventProcessedBP`
  (params (Result :type Boolean) (DeterminedValue :type Integer))
  (if Result
    _))

(event `self.FinishEvent`
  (params (Succeed :type Boolean)))

(event `self.Disapear`)

(fn `UserConstructionScript`)