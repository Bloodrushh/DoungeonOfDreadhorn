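; Base event trigger for fights, which sends the player to a table and then into combat through the DungeonManager.
; On trigger it runs the parent logic, waits briefly and moves the player into the table.
; When the event is processed, it moves the player into the fight and has the FightManager initiate it with EnemyClasses; the determined value is only printed.
; The finish handler is empty, and older event-start calls remain disconnected.
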(event `self.OnTriggered`
  (params (TriggeredActor :type "Actor Object Reference"))
  (`parent.OnTriggered` TriggeredActor)
  (`KismetSystemLibrary.PrintString` "OmTrigerred")
  (`KismetSystemLibrary.Delay` 2.0)
  (`DungeonManager.MovePlayerIntoTable` (`self.DungeonManager`)))

(event `self.OnEventProcessedBP`
  (params (Result :type Boolean) (DeterminedValue :type Integer))
  (`KismetSystemLibrary.PrintString` (`KismetStringLibrary.Concat_StrStr` "EventTriggerFight::Event ProcessedBP. Determined value: " (`KismetStringLibrary.Conv_IntToString` DeterminedValue)) true true (struct :`G` 0.66 :`B` 1.0 :`A` 1.0) 5.0)
  (`DungeonManager.MovePlayerIntoFight` (`self.DungeonManager`))
  (`FightManager.InitiateFight` (`DungeonManager.FightManager` (`self.DungeonManager`)) (make `FightInitiateInfo` (`self.Enemy Classes`))))

(event `self.OnEventFinishedBP`)

(fn `UserConstructionScript`)