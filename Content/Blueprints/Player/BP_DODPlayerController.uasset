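; Player controller that switches possession between the dungeon pawn it starts with and a board pawn.
; On BeginPlay it caches the controlled pawn, plus the first board pawn and first dice actor found in the level.
; Keys 1 and 2 possess the board and dungeon pawns respectively, hiding each swap behind a delayed camera fade.
; Returning to the dungeon also resets the dice before possession.
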(event `self.ReceiveBeginPlay`
  (set `self.BPDungeonPawn` (`self.K2_GetPawn`))
  (bind _outactors (`GameplayStatics.GetAllActorsOfClass` "/Script/DongeonOfDreadhorn.BoardPawn"))
  (set `self.BPBoardPawn` (`|GetArrayItem` _outactors))
  (bind _outactors_2 (`GameplayStatics.GetAllActorsOfClass` "/Game/Blueprints/Board/BP_DiceBase.BP_DiceBase_C"))
  (set `self.BP_Dice` (`|GetArrayItem` _outactors_2)))

(event `Key|One`
  (params (Key :type "Key Structure"))
  (:`Pressed`
    (`PlayerCameraManager.StartCameraFade` :`self` (`self.PlayerCameraManager`) :`ToAlpha` 1.0 :`Duration` 1.0 :`bHoldWhenFinished` true)
    (`KismetSystemLibrary.Delay` 2.0)
    (`self.Possess` (`self.BPBoardPawn`))
    (`PlayerCameraManager.StartCameraFade` :`self` (`self.PlayerCameraManager`) :`FromAlpha` 1.0 :`Duration` 1.0)))

(event `Key|Two`
  (params (Key :type "Key Structure"))
  (:`Pressed`
    (`PlayerCameraManager.StartCameraFade` :`self` (`self.PlayerCameraManager`) :`ToAlpha` 1.0 :`Duration` 1.0 :`bHoldWhenFinished` true)
    (`KismetSystemLibrary.Delay` 2.0)
    (`/Game/Blueprints/Board/BP_DiceBase.Reset` (`self.BP_Dice`))
    (`self.Possess` (`self.BPDungeonPawn`))
    (`PlayerCameraManager.StartCameraFade` :`self` (`self.PlayerCameraManager`) :`FromAlpha` 1.0 :`Duration` 1.0)))

(fn `UserConstructionScript`)