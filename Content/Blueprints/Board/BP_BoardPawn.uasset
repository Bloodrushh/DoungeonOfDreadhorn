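; BP_BoardPawn is a board pawn that switches motion controller tracking for its two hands on and off with possession.
; On possession it activates the MotionController of LeftHand and RightHand without a reset, and on unpossession it deactivates both.
; Both events act only when both hand references are valid, and the construction script is empty.
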(event `self.ReceivePossessed`
  (params (NewController :type "Controller Object Reference"))
  (if (and (`KismetSystemLibrary.IsValid` (`self.LeftHand`)) (`KismetSystemLibrary.IsValid` (`self.RightHand`)))
    (`ActorComponent.Activate` (`HandBase.MotionController` (`self.LeftHand`)) false)
    (`ActorComponent.Activate` (`HandBase.MotionController` (`self.RightHand`)) false)))

(event `self.ReceiveUnpossessed`
  (params (OldController :type "Controller Object Reference"))
  (if (and (`KismetSystemLibrary.IsValid` (`self.LeftHand`)) (`KismetSystemLibrary.IsValid` (`self.RightHand`)))
    (`ActorComponent.Deactivate` (`HandBase.MotionController` (`self.LeftHand`)))
    (`ActorComponent.Deactivate` (`HandBase.MotionController` (`self.RightHand`)))))

(fn `UserConstructionScript`)