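; BP_FightManager manages a fight encounter, spawning its enemies and supplying the player's teleport location.
; SpawnEnemies blocking-loads each enemy class from the passed info and spawns it at the matching local spawn point, facing the teleport location.
; Each enemy receives the player pawn and manager references, then is registered as a participant.
; BeginFight only defers to the parent, and GetTeleportLocation converts a local point to world space with a debug print.
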(event `self.BeginFight`
  (`parent.BeginFight`))

(event `self.SpawnEnemies`
  (params (Info :type "FightInitiateInfo Structure"))
  (for (_array_element _array_index) (`.EnemyClasses` (break `FightInitiateInfo` Info))
    (bind _returnvalue (`KismetSystemLibrary.LoadClassAsset_Blocking` _array_element))
    (bind _asbp_enemy_base (castclass `/Game/Blueprints/Enemies/BP_EnemyBase` _returnvalue))
    (bind _returnvalue_2 (`KismetMathLibrary.TransformLocation` (`self.GetTransform`) (`|GetArrayItem` (`self.EnemiesSpawnPoints`) _array_index)))
    (bind _returnvalue_3 (`|SpawnActorFromClass` _asbp_enemy_base (`KismetMathLibrary.MakeTransform` _returnvalue_2 (`KismetMathLibrary.FindLookAtRotation` _returnvalue_2 (`self.GetTeleportLocation`))) "AlwaysSpawn" "OverrideRootScale" null (`self.PlayerPawn`) self null))
    (`self.AddParticipant` _returnvalue_3)))

(fn `GetTeleportLocation`
  (returns (ReturnValue :type "Vector Structure"))
  (`KismetSystemLibrary.PrintString` "FightManager:: GetTeleportLocation")
  (return (`KismetMathLibrary.TransformLocation` (`self.GetTransform`) (`self.PlayerTeleportLocation`))))

(fn `UserConstructionScript`)