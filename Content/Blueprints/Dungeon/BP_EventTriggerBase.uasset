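; Dungeon event trigger that starts a table event once, when an overlapping actor passes a line-of-sight check.
; It sends its EventInfo and a result callback to the first BP_TableBase found in the level, then prints the event details on screen.
; The callback prints a colored success or failure message and destroys the trigger; it applies no effects itself.
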(event `self.ReceiveBeginPlay`)

(event `self.ReceiveActorBeginOverlap`
  (params (OtherActor :type "Actor Object Reference"))
  (bind (_event _battributebased _attribute _breversed _successnumbers _successeffect _successattribute _successamount _faileffect _failattribute _failamount) (break `EventInfo` (`self.EventInfo`)))
  (bind _returnvalue (`self.TargetIsOnLineOfSight` OtherActor))
  (if _returnvalue
    (`/Engine/EditorBlueprintResources/StandardMacros.DoOnce` false
      (:`Completed`
        (bind _outactors (`GameplayStatics.GetAllActorsOfClass` "/Game/Blueprints/Board/BP_TableBase.BP_TableBase_C"))
        (`TableBase.StartEvent` (`|GetArrayItem` _outactors) (`self.EventInfo`) (delegate `CustomEvent_0`))
        (`KismetSystemLibrary.PrintString` (`KismetStringLibrary.Concat_StrStr` "Event has been started. Info:" "Type: " (`|GetEnumeratorNameAsString` _event) " | Success effect: " (`|GetEnumeratorNameAsString` _successeffect) " | Success attribute: " (`|GetEnumeratorNameAsString` _successattribute) " | Success amount: " (`KismetStringLibrary.Conv_IntToString` _successamount) " | Fail effect: " (`|GetEnumeratorNameAsString` _faileffect) " | Fail attribute: " (`|GetEnumeratorNameAsString` _failattribute) " | Fail amount: " (`KismetStringLibrary.Conv_IntToString` _failamount)) true true (struct :`R` 0.91836 :`G` 1.0 :`A` 1.0) 11.0)))))

(event `CustomEvent_0`
  (params (bSucceed :type Boolean))
  (`KismetSystemLibrary.PrintString` (select `bool` bSucceed :`false` "You are RAK. SOSI" :`true` "You are Lucky!") true true (`KismetMathLibrary.SelectColor` (struct :`G` 1.0 :`B` 0.174918 :`A` 1.0) (struct :`R` 1.0 :`B` 0.169777 :`A` 1.0) bSucceed) 11.0)
  (`self.K2_DestroyActor`))

(fn `UserConstructionScript`)